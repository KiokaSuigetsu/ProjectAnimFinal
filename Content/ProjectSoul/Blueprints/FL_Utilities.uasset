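; FL_Utilities is a utility library whose ReductionDamage function applies a defense value to incoming damage against HP.
; Non-negative defense scales damage by 100/(100+Defense), giving diminishing returns.
; Negative defense selects (2−100)/(100−Defense) as written, a negative multiplier that makes positive damage raise HP.
; It returns remaining HP without clamping, the scaled damage, and a reduction percentage computed as multiplier times defense.
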(fn ReductionDamage
  (params (Value%20Hp :type Float%20%28double-precision%29) (DamageAfterSoustract :type Float%20%28double-precision%29) (ValueDefense :type Float%20%28double-precision%29))
  (bind _returnvalue (+ 1e+02 ValueDefense))
  (bind _returnvalue_2 (< ValueDefense 0.0))
  (bind _returnvalue_3 (- 1e+02 ValueDefense))
  (bind _returnvalue_4 (- 2.0 1e+02))
  (bind _returnvalue_5 (Math|Float|SelectFloat _returnvalue_3 _returnvalue _returnvalue_2))
  (bind _returnvalue_6 (/ 1e+02 _returnvalue_5))
  (bind _returnvalue_7 (/ _returnvalue_4 _returnvalue_5))
  (bind _returnvalue_8 (Math|Float|SelectFloat _returnvalue_7 _returnvalue_6 _returnvalue_2))
  (bind _returnvalue_9 (* DamageAfterSoustract _returnvalue_8))
  (return (- Value%20Hp _returnvalue_9) _returnvalue_9 (* _returnvalue_8 ValueDefense)))