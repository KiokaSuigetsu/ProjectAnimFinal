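; Boss arena blocker that traps the player in an encounter until the referenced AI is killed.
; When the overlap with the BoxEnter volume ends, a DoOnce fires, and if the leaving actor is BP_Player the box switches to block all channels.
; It binds to the referenced AI's damage event on BeginPlay and destroys itself once that AI's Hp reaches zero or below.
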(event OnComponentEndOverlap(BoxEnter)
  (params (OverlappedComponent :type Primitive%20Component%20Object%20Reference) (OtherActor :type Actor%20Object%20Reference) (OtherComp :type Primitive%20Component%20Object%20Reference) (OtherBodyIndex :type Integer))
  (Utilities|FlowControl|DoOnce false
    (:Completed
      (Utilities|Casting|CastToBP_Player OtherActor)
      (Collision|SetCollisionResponsetoAllChannels (Variables|Default|GetBoxEnter) "ECR_Block"))))

(event Custom|Dead
  (params (DamagedActor :type Actor%20Object%20Reference) (Damage :type Float%20%28single-precision%29) (DamageType :type Damage%20Type%20Object%20Reference) (InstigatedBy :type Controller%20Object%20Reference) (DamageCauser :type Actor%20Object%20Reference))
  (if (<= (Variables|/Game/ProjectSoul/Blueprints/IA/Bp_MainIA.Bp_MainIA_C|GetHp (stale EventBeginPlay _refia)) 0.0)
    (Actor|DestroyActor)))

(event EventBeginPlay
  (bind _refia (Variables|Default|GetRefIa)
    (:then
      (EventDispatchers|BindEventtoOnTakeAnyDamage _refia (delegate Custom|Dead)))
    (:else)))

(fn ConstructionScript)