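; Flying mage boss that, once activated, hands the player to its AIC_Mage controller, takes flight and turns toward them on a looping timer.
; Timelines move the mesh for flight, descent and ascension, and can refill HP.
; Attacks include a Niagara laser with timer-driven sphere-trace damage and projectiles spawned with movement deactivated.
; At zero HP it notifies the controller, then plays a down montage, or dies and is destroyed if P2 is set.
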(event Custom|ActivateBoss
  (params (PlayerRef :type BP%20Player%20Object%20Reference))
  (Variables|Default|SetBossActivate? true)
  (bind _output_get (Variables|Default|SetPlayerRef PlayerRef))
  (bind _output_get_2 (Variables|Default|SetAs%20AIC%20Mage (.AsAIC%20Mage (Utilities|Casting|CastToAIC_Mage (AI|GetAIController self)))))
  (Default|BeginBoss _output_get_2 _output_get)
  (CallFunction|RotatePlayer 0.001)
  (CallFunction|Fly true))

(event Custom|RotatePlayer
  (params (Time :type Float%20%28single-precision%29))
  (bind _returnvalue (Utilities|Time|SetTimerbyEvent (delegate Custom|Rotate) Time true))
  (Variables|Default|SetTimerRotate _returnvalue))

(event Custom|Ascension
  (params (B :type Vector :default "0.000000,0.000000,600.000000"))
  (bind _lerp (Timeline|Timeline Play)
    (:Update
      (Transformation|SetRelativeLocation (Variables|Character|GetMesh) (Math|Vector|Lerp(Vector) "0.000000,0.000000,50.000000" B _lerp) false false))))

(event Custom|DownMesh
  (bind _lerp (Timeline|Down Play)
    (:Update
      (Transformation|SetRelativeLocation (Variables|Character|GetMesh) (Math|Vector|Lerp(Vector) "0.000000,0.000000,50.000000" "0.000000,0.000000,-151.000000" _lerp) false false))))

(event Custom|ReverseDownMesh
  (bind _lerp (Timeline|Down Reverse)
    (:Update
      (Transformation|SetRelativeLocation (Variables|Character|GetMesh) (Math|Vector|Lerp(Vector) "0.000000,0.000000,50.000000" "0.000000,0.000000,-151.000000" _lerp) false false))))

(event Custom|SpawnProjectileP32
  (params (Target :type Scene%20Component%20Object%20Reference))
  (Math|Integer|IncrementInt (Variables|Default|GetCount)
    (:%20%20
      (bind _returnvalue (Game|SpawnActorfromClass "/Game/ProjectSoul/Blueprints/IA/Boss/Mage/Bp/Bp_Projectile32.Bp_Projectile32_C" (Math|Transform|MakeTransform (Transformation|GetWorldLocation Target) (Transformation|GetWorldRotation Target) "0.100000,0.100000,0.100000") "AlwaysSpawn" "MultiplyWithRoot" 0 4e+02 5e+03 6e+03 3.7e+04 "/Game/sA_Megapack_v1/sA_Projectilevfx/Vfx/Fx/Niagara_Systems/NS_Projectile6.NS_Projectile6" "/Game/sA_Megapack_v1/sA_StylizedAttacksPack/FX/NiagaraSystems/NS_Flame_Trail.NS_Flame_Trail" 5e+02 0))
      (Utilities|Array|Add (Variables|Default|GetProjectileCast32) _returnvalue)
      (Components|Activation|Deactivate (Variables|/Game/ProjectSoul/Blueprints/IA/Boss/Mage/Bp/Bp_Projectile32.Bp_Projectile32_C|GetProjectileMovement _returnvalue)))))

(event Custom|RotateArrow
  (for _array_element (Utilities|Array|MakeArray (Variables|Default|GetArrow1) (Variables|Default|GetArrow2) (Variables|Default|GetArrow3))
    (Transformation|SetWorldRotation _array_element (Math|Rotator|FindLookatRotation (Transformation|GetWorldLocation _array_element) (Transformation|GetActorLocation (Variables|Default|GetPlayerRef))) false false)))

(event Custom|UpHp
  (bind _lerp (Timeline|HpLerp Play)
    (:Update
      (Variables|Default|SetHp (Math|Float|Lerp 0.0 (Variables|Default|GetHpMax) _lerp)))))

(event Custom|SpawnProjectileP31
  (bind _arrow1 (Variables|Default|GetArrow1))
  (bind _returnvalue (Game|SpawnActorfromClass "/Game/ProjectSoul/Blueprints/IA/Boss/Mage/Bp/Bp_ProjectileShuriken.Bp_ProjectileShuriken_C" (Math|Transform|MakeTransform (Transformation|GetWorldLocation _arrow1) (Transformation|GetWorldRotation _arrow1) "0.100000,0.100000,0.100000") "AlwaysSpawn" "MultiplyWithRoot" 0 2.5e+02 5e+03 6e+03 3.5e+04 "/Game/sA_Megapack_v1/sA_Projectilevfx/Vfx/Fx/Niagara_Systems/NS_Projectile6.NS_Projectile6" "/Game/sA_Megapack_v1/sA_StylizedAttacksPack/FX/NiagaraSystems/NS_Flame_Trail.NS_Flame_Trail" 5e+02 0))
  (bind _output_get (Variables|Default|SetProjectileCast31 _returnvalue))
  (Components|Activation|Deactivate (Variables|/Game/ProjectSoul/Blueprints/IA/Boss/Mage/Bp/Bp_ProjectileShuriken.Bp_ProjectileShuriken_C|GetProjectileMovement _output_get)))

(event Custom|Rotate
  (bind _playerref (Variables|Default|GetPlayerRef)
    (:then
      (Transformation|SetActorRotation (Math|Rotator|MakeRotator (.roll (Math|Rotator|FindLookatRotation (Transformation|GetActorLocation) (Transformation|GetActorLocation _playerref))) 0.0 (.yaw (Math|Rotator|FindLookatRotation (Transformation|GetActorLocation) (Transformation|GetActorLocation _playerref))))))
    (:else)))

(event Custom|StopRotatePlayer
  (Utilities|Time|ClearandInvalidateTimerbyHandle (Variables|Default|GetTimerRotate)))

(event Custom|UnFly
  (Utilities|FlowControl|Sequence
    (:then_0
      (bind (_direction _lerp) (Timeline|FlyUp Reverse)
        (:Update
          (Transformation|SetRelativeLocation (Variables|Character|GetMesh) (Math|Vector|Lerp(Vector) "0.000000,0.000000,-151.000000" "0.000000,0.000000,50.000000" _lerp) false false))
        (:Finished
          (switch Utilities|FlowControl|Switch|SwitchonETimelineDirection _direction
            (:Forward
              (if (stale Custom|Fly Begin?)
                (Default|Set/UnSetPatrol (Variables|Default|GetAs%20AIC%20Mage) true)))))))
    (:then_1
      (Utilities|FlowControl|Delay 1.0)
      (Variables|Default|SetIsFly? false))))

(event Custom|Fly
  (params (Begin? :type Boolean))
  (Variables|Default|SetIsFly? true)
  (bind (_direction _lerp) (Timeline|FlyUp Play)
    (:Update
      (Transformation|SetRelativeLocation (Variables|Character|GetMesh) (Math|Vector|Lerp(Vector) "0.000000,0.000000,-151.000000" "0.000000,0.000000,50.000000" _lerp) false false))
    (:Finished
      (switch Utilities|FlowControl|Switch|SwitchonETimelineDirection _direction
        (:Forward
          (if Begin?
            (Default|Set/UnSetPatrol (Variables|Default|GetAs%20AIC%20Mage) true)))))))

(event Custom|Damage
  (bind (_outhit _returnvalue) (Collision|SphereTraceByChannel (Transformation|GetSocketLocation (Variables|Character|GetMesh) "handLSocket") (+ (Transformation|GetActorLocation) (* (Transformation|GetActorForwardVector) (+ (Math|Vector|Distance(Vector) (Transformation|GetActorLocation) (Transformation|GetActorLocation (Variables|Default|GetPlayerRef))) 1e+02))) 1e+02 "TraceTypeQuery3" false 0 "None"))
  (if _returnvalue
    (bind _asbp_player (Utilities|Casting|CastToBP_Player (.HitActor (Collision|BreakHitResult _outhit))))
    (Game|Damage|ApplyDamage _asbp_player 2e+01 0 0)))

(event Custom|Laser
  (bind _returnvalue (Transformation|GetActorForwardVector))
  (bind _returnvalue_2 (Transformation|GetActorLocation))
  (bind _returnvalue_3 (Transformation|GetActorLocation))
  (bind _mesh (Variables|Character|GetMesh))
  (bind _playerref (Variables|Default|GetPlayerRef))
  (bind _returnvalue_4 (Transformation|GetSocketLocation _mesh "handLSocket"))
  (bind _returnvalue_5 (Transformation|GetActorLocation _playerref))
  (bind _returnvalue_6 (Math|Vector|Distance(Vector) _returnvalue_2 _returnvalue_5))
  (bind _returnvalue_7 (+ _returnvalue_6 1e+02))
  (bind _returnvalue_8 (* _returnvalue _returnvalue_7))
  (bind _returnvalue_9 (+ _returnvalue_3 _returnvalue_8))
  (bind _returnvalue_10 (Math|Rotator|FindLookatRotation _returnvalue_4 _returnvalue_9))
  (bind _returnvalue_11 (Utilities|Time|SetTimerbyEvent (delegate Custom|Damage) 0.1 true))
  (Variables|Default|SetTimerLaser _returnvalue_11)
  (Niagara|SpawnSystematLocation "/Game/sA_Megapack_v1/sA_Rayvfx/Fx/NiagaraSystems/NS_Ray_5.NS_Ray_5" _returnvalue_4 _returnvalue_10)
  (Niagara|SpawnSystematLocation "/Game/sA_Megapack_v1/sA_Rayvfx/Fx/NiagaraSystems/NS_Energy_5.NS_Energy_5" _returnvalue_4 _returnvalue_10))

(event Custom|ReverseAscension
  (bind _lerp (Timeline|Timeline Reverse)
    (:Update
      (Transformation|SetRelativeLocation (Variables|Character|GetMesh) (Math|Vector|Lerp(Vector) "0.000000,0.000000,50.000000" (stale Custom|Ascension B) _lerp) false false))))

(event Custom|StopLaser
  (Utilities|Time|ClearandInvalidateTimerbyHandle (Variables|Default|GetTimerLaser)))

(event EventBeginPlay
  (|CallParentFunction)
  (Rendering|SetVisibility (Variables|Default|GetWings) false false)
  (Variables|Default|SetarrowTab (Utilities|Array|MakeArray (Variables|Default|GetArrow5) (Variables|Default|GetArrow2) (Variables|Default|GetArrow1) (Variables|Default|GetArrow3) (Variables|Default|GetArrow4))))

(event Collision|EventActorBeginOverlap
  (params (OtherActor :type Actor%20Object%20Reference))
  (|CallParentFunction OtherActor) ; This node is disabled and will not be called.\nDrag off pins to build functionality.
)

(event EventTick
  (params (DeltaSeconds :type Float%20%28single-precision%29))
  (|CallParentFunction DeltaSeconds) ; This node is disabled and will not be called.\nDrag off pins to build functionality.
)

(event Game|Damage|EventAnyDamage
  (params (Damage :type Float%20%28single-precision%29) (DamageType :type Damage%20Type%20Object%20Reference) (InstigatedBy :type Controller%20Object%20Reference) (DamageCauser :type Actor%20Object%20Reference))
  (if (Variables|Default|GetCanBeDamaged?)
    (bind _output_get (Variables|Default|SetHp (.DamageFinalResult (CallFunction|ReductionDamage (Variables|Default|GetHp) Damage (Variables|Default|GetDefense)))))
    (if (<= _output_get 0.0)
      (Default|Dead (Variables|Default|GetAs%20AIC%20Mage) true)
      (if (Variables|Default|GetP2?)
        (Variables|Default|SetDeath? true)
        (Animation|Montage|PlayMontage (Variables|Character|GetMesh) "/Game/ProjectSoul/Animation/Retargeter/AnimRetargeter/FlyingMagedead_Montage.FlyingMagedead_Montage"
          (:OnCompleted
            (Actor|DestroyActor)))
        (else
          (Variables|Default|SetStun? false)
          (Variables|Default|SetAsecension? false)
          (Variables|Default|SetCanBeDamaged? false)
          (CallFunction|StopRotatePlayer)
          (Animation|Montage|PlayMontage (Variables|Character|GetMesh) "/Game/ProjectSoul/Animation/Retargeter/AnimRetargeter/FlyingMagedown_Montage.FlyingMagedown_Montage")))
      (else
        (Animation|Montage|PlayMontage (Variables|Character|GetMesh) "/Game/ProjectSoul/Animation/Retargeter/AnimRetargeter/FlyingMageattacked_b_Montage.FlyingMageattacked_b_Montage")))))

(fn ConstructionScript
  (|CallParentFunction))