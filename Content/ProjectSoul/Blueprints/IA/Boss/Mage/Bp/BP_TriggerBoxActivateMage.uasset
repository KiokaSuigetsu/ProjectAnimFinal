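; Trigger box actor that starts the Mage boss encounter when the player walks into it.
; On the first player overlap, it links the player and boss references both ways by calling ActivateBoss with the player.
; It then plays the boss soundtrack from an offset start time, keeps the sound reference, and adds a boss health bar widget to the viewport, stored on the boss.
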(event OnComponentBeginOverlap(Box)
  (params (OverlappedComponent :type Primitive%20Component%20Object%20Reference) (OtherActor :type Actor%20Object%20Reference) (OtherComp :type Primitive%20Component%20Object%20Reference) (OtherBodyIndex :type Integer) (bFromSweep :type Boolean) (SweepResult :type Hit%20Result%20Structure%20%28by%20ref%29))
  (bind _asbp_player (Utilities|Casting|CastToBP_Player OtherActor))
  (Utilities|DoOnce false
    (:Completed
      (bind _refboss (Variables|Default|GetRefBoss)
        (:then
          (Variables|/Game/ProjectSoul/Blueprints/Player/BP_Player.BP_Player_C|SetRefBoss _asbp_player _refboss)
          (Default|ActivateBoss _refboss _asbp_player)
          (bind _returnvalue (Audio|SpawnSound2D (Variables|Default|GetOstBoss) 0.5 1.0 2.4e+02 0))
          (Variables|Default|SetSoundRef _returnvalue)
          (bind _returnvalue_2 (UserInterface|CreateWidget "/Game/ProjectSoul/Widget/WBP_BossHealthBar.WBP_BossHealthBar_C" 0 _refboss))
          (bind _output_get (Variables|/Game/ProjectSoul/Blueprints/IA/Boss/Bp_MainBoss.Bp_MainBoss_C|SetRefWidgetHp _refboss _returnvalue_2))
          (UserInterface|Viewport|AddtoViewport _output_get 0))
        (:else)))))

(event EventBeginPlay)

(event Collision|EventActorBeginOverlap
  (params (OtherActor :type Actor%20Object%20Reference)))

(event EventTick
  (params (DeltaSeconds :type Float%20%28single-precision%29)))

(fn ConstructionScript)