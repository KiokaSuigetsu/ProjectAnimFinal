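; Homing projectile for the Mage boss that explodes on impact and leaves a Bp_Zone behind.
; On BeginPlay it applies its speed and homing settings and targets the player's capsule; Tick switches homing off once it gets close to the player.
; A player hit applies damage and spawns AOE effects and the zone at the mesh; other hits trace down to place them below the impact, then the projectile destroys itself.
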(event OnComponentHit(Box)
  (params (HitComponent :type Primitive%20Component%20Object%20Reference) (OtherActor :type Actor%20Object%20Reference) (OtherComp :type Primitive%20Component%20Object%20Reference) (NormalImpulse :type Vector :default "0, 0, 0") (Hit :type Hit%20Result%20Structure%20%28by%20ref%29))
  (bind _asbp_player (Utilities|Casting|CastToBP_Player OtherActor)
    (:then
      (Game|Damage|ApplyDamage _asbp_player (Variables|Default|GetBase%20Damage) 0 0)
      (Niagara|SpawnSystematLocation "/Game/Market/sA_Megapack_v1/sA_StylizedAttacksPack/FX/NiagaraSystems/NS_AOE_Attack_1.NS_AOE_Attack_1" (Transformation|GetWorldLocation (Variables|/Script/Engine.Character|GetMesh _asbp_player)))
      (Niagara|SpawnSystematLocation "/Game/Market/sA_Megapack_v1/sA_StylizedAttacksPack/FX/NiagaraSystems/NS_AOE_Explosion_1.NS_AOE_Explosion_1" (Transformation|GetWorldLocation (Variables|/Script/Engine.Character|GetMesh _asbp_player)))
      (Game|SpawnActorfromClass "/Game/ProjectSoul/Blueprints/IA/Boss/Mage/Bp/Bp_Zone.Bp_Zone_C" (Math|Transform|MakeTransform (Transformation|GetWorldLocation (Variables|/Script/Engine.Character|GetMesh _asbp_player)) "0, 0, 0" "2.000000,2.000000,2.000000") "AlwaysSpawn" "MultiplyWithRoot" 0 0))
    (:CastFailed
      (bind _outhit (Collision|LineTraceByChannel (.location Hit) (- (.location Hit) "0.000000,0.000000,5000.000000") "TraceTypeQuery1" false 0 "None"))
      (Niagara|SpawnSystematLocation "/Game/Market/sA_Megapack_v1/sA_StylizedAttacksPack/FX/NiagaraSystems/NS_AOE_Attack_1.NS_AOE_Attack_1" (.location _outhit) "0, 0, 0" "10.000000,10.000000,10.000000")
      (Niagara|SpawnSystematLocation "/Game/Market/sA_Megapack_v1/sA_StylizedAttacksPack/FX/NiagaraSystems/NS_AOE_Explosion_1.NS_AOE_Explosion_1" (.location _outhit))
      (Game|SpawnActorfromClass "/Game/ProjectSoul/Blueprints/IA/Boss/Mage/Bp/Bp_Zone.Bp_Zone_C" (Math|Transform|MakeTransform (.location _outhit) "0, 0, 0" "2.000000,2.000000,2.000000") "AlwaysSpawn" "MultiplyWithRoot" 0 0)))
  (Actor|DestroyActor))

(event EventBeginPlay
  (bind _returnvalue (Game|GetPlayerCharacter 0))
  (bind _projectilemovement (Variables|Default|GetProjectileMovement))
  (bind _projectilemovement_2 (Variables|Default|GetProjectileMovement))
  (bind _asbp_player (Utilities|Casting|CastToBP_Player _returnvalue))
  (Variables|/Script/Engine.ProjectileMovementComponent|SetInitialSpeed _projectilemovement (Variables|Default|GetInitial%20Speed))
  (Variables|/Script/Engine.ProjectileMovementComponent|SetMaxSpeed _projectilemovement (Variables|Default|GetMax%20Speed))
  (Variables|/Script/Engine.ProjectileMovementComponent|SetHomingAccelerationMagnitude _projectilemovement_2 (Variables|Default|GetHoming%20Acceleration%20Magnitude))
  (Variables|Default|SetAs%20BP%20Player _asbp_player)
  (Variables|/Script/Engine.ProjectileMovementComponent|SetHomingTargetComponent _projectilemovement_2 (Variables|/Script/Engine.Character|GetCapsuleComponent _asbp_player)))

(event EventTick
  (params (DeltaSeconds :type Float%20%28single-precision%29))
  (bind _projectilemovement (Variables|Default|GetProjectileMovement))
  (Utilities|IsValid _projectilemovement
    (:Is%20Valid
      (if (< (Math|Vector|Distance(Vector) (Transformation|GetActorLocation) (Transformation|GetActorLocation (Variables|Default|GetAs%20BP%20Player))) 2e+02)
        (Variables|/Script/Engine.ProjectileMovementComponent|SetbIsHomingProjectile _projectilemovement false)))))

(fn ConstructionScript)