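; Mage boss actor that, once activated, turns to face the player and takes to the air.
; ActivateBoss stores the player, hands it to the AIC_Mage controller, then starts rotation and flight.
; A near-per-frame looping timer applies full look-at rotation until StopRotatePlayer clears it.
; The FlyUp timeline raises only the mesh and enables patrol on finish; UnFly reverses it and clears IsFly after a delay.
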(event Custom|ActivateBoss
  (params (PlayerRef :type BP%20Player%20Object%20Reference))
  (Variables|Default|SetBossActivate? true)
  (bind _output_get (Variables|Default|SetPlayerRef PlayerRef))
  (bind _output_get_2 (Variables|Default|SetAs%20AIC%20Mage (.AsAIC%20Mage (Utilities|Casting|CastToAIC_Mage (AI|GetAIController self)))))
  (Default|BeginBoss _output_get_2 _output_get)
  (CallFunction|RotatePlayer)
  (CallFunction|Fly))

(event Custom|RotatePlayer
  (bind _returnvalue (Utilities|Time|SetTimerbyEvent (delegate Custom|Rotate) 0.001 true))
  (Variables|Default|SetTimerRotate _returnvalue))

(event Custom|Rotate
  (bind _playerref (Variables|Default|GetPlayerRef)
    (:then
      (Transformation|SetActorRotation (Math|Rotator|MakeRotator (.roll (Math|Rotator|FindLookatRotation (Transformation|GetActorLocation) (Transformation|GetActorLocation _playerref))) (.pitch (Math|Rotator|FindLookatRotation (Transformation|GetActorLocation) (Transformation|GetActorLocation _playerref))) (.yaw (Math|Rotator|FindLookatRotation (Transformation|GetActorLocation) (Transformation|GetActorLocation _playerref))))))
    (:else)))

(event Custom|StopRotatePlayer
  (Utilities|Time|ClearandInvalidateTimerbyHandle (Variables|Default|GetTimerRotate)))

(event Custom|UnFly
  (Utilities|FlowControl|Sequence
    (:then_0
      (bind _lerp (Timeline|FlyUp Reverse)
        (:Update
          (Transformation|SetRelativeLocation (Variables|Character|GetMesh) (Math|Vector|Lerp(Vector) "0.000000,0.000000,-151.000000" "0.000000,0.000000,50.000000" _lerp) false false))
        (:Finished
          (Default|Set/UnSetPatrol (Variables|Default|GetAs%20AIC%20Mage) true))))
    (:then_1
      (Utilities|FlowControl|Delay 1.0)
      (Variables|Default|SetIsFly? false))))

(event Custom|Fly
  (Variables|Default|SetIsFly? true)
  (bind _lerp (Timeline|FlyUp Play)
    (:Update
      (Transformation|SetRelativeLocation (Variables|Character|GetMesh) (Math|Vector|Lerp(Vector) "0.000000,0.000000,-151.000000" "0.000000,0.000000,50.000000" _lerp) false false))
    (:Finished
      (Default|Set/UnSetPatrol (Variables|Default|GetAs%20AIC%20Mage) true))))

(event EventBeginPlay
  (|CallParentFunction) ; This node is disabled and will not be called.\nDrag off pins to build functionality.
)

(event Collision|EventActorBeginOverlap
  (params (OtherActor :type Actor%20Object%20Reference))
  (|CallParentFunction OtherActor) ; This node is disabled and will not be called.\nDrag off pins to build functionality.
)

(event EventTick
  (params (DeltaSeconds :type Float%20%28single-precision%29))
  (|CallParentFunction DeltaSeconds) ; This node is disabled and will not be called.\nDrag off pins to build functionality.
)

(fn ConstructionScript
  (|CallParentFunction))