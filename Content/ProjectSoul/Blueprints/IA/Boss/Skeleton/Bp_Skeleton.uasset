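; Skeleton boss Blueprint that wakes up on activation and turns to face the player.
; ActivateBoss stores the player reference, plays a 2D sound, passes activation to the AIC_SKeleton AI controller and starts the rotation.
; A fast looping timer, used instead of Tick, applies the roll and yaw of the look-at rotation toward the player until StopRotatePlayer clears it.
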(event Custom|ActivateBoss
  (params (PlayerRef :type BP%20Player%20Object%20Reference))
  (Variables|Default|SetBossActivate? true)
  (bind _output_get (Variables|Default|SetPlayerRef PlayerRef))
  (Audio|PlaySound2D 0 1.0 1.0 0.0 0 0)
  (Default|ActivateBoss (.AsAIC%20SKeleton (Utilities|Casting|CastToAIC_SKeleton (AI|GetAIController self))) _output_get)
  (CallFunction|RotatePlayer))

(event Custom|RotatePlayer
  ;[1 1 1] Set/Unset Player to Rotation
  (bind _returnvalue (Utilities|Time|SetTimerbyEvent (delegate Custom|Rotate) 0.001 true))
  (Variables|Default|SetTimerRotate _returnvalue))

(event Custom|Rotate
  ;[1 1 1] Set/Unset Player to Rotation
  (bind _playerref (Variables|Default|GetPlayerRef)
    (:then
      (Transformation|SetActorRotation (Math|Rotator|MakeRotator (.roll (Math|Rotator|FindLookatRotation (Transformation|GetActorLocation) (Transformation|GetActorLocation _playerref))) 0.0 (.yaw (Math|Rotator|FindLookatRotation (Transformation|GetActorLocation) (Transformation|GetActorLocation _playerref))))))
    (:else)))

(event Custom|StopRotatePlayer
  ;[1 1 1] Set/Unset Player to Rotation
  (Utilities|Time|ClearandInvalidateTimerbyHandle (Variables|Default|GetTimerRotate)))

(event EventBeginPlay
  (|CallParentFunction))

(event Collision|EventActorBeginOverlap
  (params (OtherActor :type Actor%20Object%20Reference))
  (|CallParentFunction OtherActor) ; This node is disabled and will not be called.\nDrag off pins to build functionality.
)

(event EventTick
  (params (DeltaSeconds :type Float%20%28single-precision%29))
  (|CallParentFunction DeltaSeconds) ; This node is disabled and will not be called.\nDrag off pins to build functionality.
)

(fn ConstructionScript
  (|CallParentFunction))