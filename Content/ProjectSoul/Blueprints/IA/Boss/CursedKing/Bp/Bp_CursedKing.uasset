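; Cursed King boss character that activates its AI controller with a talk sound and tracks the player through a looping rotation timer.
; Its ultimate uses timelines to leap in flying mode, then dive near the player's saved location, with a separate traced Niagara shockwave event.
; It also throws Atk-scaled spears at the player.
; Damage is reduced by defense, triggering optional hit montages or a death sequence that ends the boss bar.
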(event Custom|ActivateBoss
  (params (PlayerRef :type BP%20Player%20Object%20Reference))
  ;[1 1 1] Ultimate
  (Variables|Default|SetBossActivate? true)
  (bind _output_get (Variables|Default|SetPlayerRef PlayerRef))
  (bind _output_get_2 (Variables|Default|SetAs%20AIC%20Boss%20Cursed%20King (.AsAIC%20Boss%20Cursed%20King (Utilities|Casting|CastToAIC_BossCursedKing (AI|GetAIController self)))))
  (Audio|PlaySound2D "/Game/ProjectSoul/Sound/CursedTalk.CursedTalk" 1.0 1.0 0.0 0 0)
  (Default|BeginBoss _output_get_2 _output_get)
  (CallFunction|RotatePlayer))

(event Custom|RotatePlayer
  ;[1 1 1] Set/Unset Player to Rotation
  (bind _returnvalue (Utilities|Time|SetTimerbyEvent (delegate Custom|Rotate) 0.001 true))
  (Variables|Default|SetTimerRotate _returnvalue))

(event Custom|Rotate
  ;[1 1 1] Set/Unset Player to Rotation
  (bind _playerref (Variables|Default|GetPlayerRef)
    (:then
      (Transformation|SetActorRotation (Math|Rotator|MakeRotator (.roll (Math|Rotator|FindLookatRotation (Transformation|GetActorLocation) (Transformation|GetActorLocation _playerref))) 0.0 (.yaw (Math|Rotator|FindLookatRotation (Transformation|GetActorLocation) (Transformation|GetActorLocation _playerref))))))
    (:else)))

(event Custom|StopRotatePlayer
  ;[1 1 1] Set/Unset Player to Rotation
  (Utilities|Time|ClearandInvalidateTimerbyHandle (Variables|Default|GetTimerRotate)))

(event Custom|JumpPoint
  (bind _returnvalue (Transformation|GetActorForwardVector))
  (bind _returnvalue_2 (Transformation|GetActorLocation))
  (bind _returnvalue_3 (* _returnvalue 5e+02))
  (bind _returnvalue_4 (+ _returnvalue_3 _returnvalue_2))
  (bind _returnvalue_5 (+ (.z _returnvalue_4) 4e+02))
  (bind _returnvalue_6 (Math|Vector|MakeVector (.x _returnvalue_4) (.y _returnvalue_4) _returnvalue_5))
  ;[1 1 1] Ultimate
  (bind (_outhit _returnvalue_7) (Collision|LineTraceByChannel _returnvalue_6 _returnvalue_6 "TraceTypeQuery1" false 0 "None"))
  (Pawn|Components|CharacterMovement|SetMovementMode (Variables|Character|GetCharacterMovement) "MOVE_Flying" 0)
  (bind _z (Timeline|JumpZ Play)
    (:Update
      (Transformation|SetActorLocation (Math|Vector|Lerp(Vector) (Transformation|GetActorLocation) (Math|Vector|SelectVector (.location _outhit) (.traceend _outhit) _returnvalue_7) _z) true false))))

(event Custom|Down
  ;[1 1 1] Ultimate
  (CallFunction|StopRotatePlayer)
  (Variables|Default|SetLocationPlayer (Transformation|GetActorLocation (Game|GetPlayerCharacter 0)))
  (Variables|Default|SetAttackmidHp? false)
  (bind _locationplayerlerp (Timeline|GoOnPlayer Play)
    (:Update
      (Transformation|SetActorLocation (Math|Vector|Lerp(Vector) (Transformation|GetActorLocation) (Math|Vector|MakeVector (- (.x (Variables|Default|GetLocationPlayer)) 3e+02) (.y (Variables|Default|GetLocationPlayer)) (+ (.z (Variables|Default|GetLocationPlayer)) 1e+02)) _locationplayerlerp) false false))
    (:Finished
      (Pawn|Components|CharacterMovement|SetMovementMode (Variables|Character|GetCharacterMovement) "MOVE_Walking" 0))))

(event Custom|SpawnProjectile
  (bind _returnvalue (Game|GetPlayerCharacter 0))
  (bind _mesh (Variables|Character|GetMesh))
  (bind _returnvalue_2 (Transformation|GetSocketLocation _mesh "SpearSocket"))
  (bind _returnvalue_3 (Transformation|GetActorLocation _returnvalue))
  ;[1 1 1] SpawnSpear
  (Game|SpawnActorfromClass "/Game/ProjectSoul/Blueprints/IA/Boss/CursedKing/Bp/Bp_Projectile.Bp_Projectile_C" (Math|Transform|MakeTransform _returnvalue_2 (Math|Rotator|FindLookatRotation _returnvalue_2 (Math|Vector|MakeVector (.x _returnvalue_3) (.y _returnvalue_3) (+ (.z _returnvalue_3) -85.0))) "1.000000,1.000000,1.000000") "AlwaysSpawn" "MultiplyWithRoot" 0 (* (Variables|Default|GetAtk) 1.5) 0)
  (Rendering|SetVisibility (Variables|Default|GetNiagara) false false))

(event Custom|SpawnParticle
  (bind _niagara (Variables|Default|GetNiagara))
  ;[1 1 1] SpawnSpear
  (Rendering|SetVisibility _niagara true false)
  (Components|Activation|Activate _niagara false))

(event Custom|SpawnNiagaraExplosion
  (bind _locationplayer (Variables|Default|GetLocationPlayer))
  (bind _returnvalue (+ (.z _locationplayer) 1e+02))
  (bind _returnvalue_2 (- (.x _locationplayer) 3e+02))
  (bind _returnvalue_3 (Math|Vector|MakeVector _returnvalue_2 (.y _locationplayer) _returnvalue))
  ;[1 1 1] Ultimate
  (bind _outhit (Collision|LineTraceByChannel _returnvalue_3 (- _returnvalue_3 "0.000000,0.000000,500.000000") "TraceTypeQuery1" false 0 "None"))
  (Niagara|SpawnSystematLocation "/Game/ProjectSoul/Particle/ShockWave/NS_ShowWave.NS_ShowWave" (+ (.location _outhit) "0.000000,0.000000,0.100000")))

(event Game|Damage|EventAnyDamage
  (params (Damage :type Float%20%28single-precision%29) (DamageType :type Damage%20Type%20Object%20Reference) (InstigatedBy :type Controller%20Object%20Reference) (DamageCauser :type Actor%20Object%20Reference))
  ;[1 1 1] TakeDamage
  (if (not (Variables|Default|GetDeath?))
    (bind _output_get (Variables|Default|SetHp (.DamageFinalResult (CallFunction|ReductionDamage (Variables|Default|GetHp) Damage (Variables|Default|GetDefense)))))
    (Development|PrintString (Utilities|String|Append "Damage :" (Utilities|String|ToString(Float) (.DamageCalculate (CallFunction|ReductionDamage (Variables|Default|GetHp) Damage (Variables|Default|GetDefense)))) "   ReductionDamage" (Utilities|String|ToString(Float) (.DamageReductionPourcentage (CallFunction|ReductionDamage (Variables|Default|GetHp) Damage (Variables|Default|GetDefense)))) "%"))
    (if (Variables|Default|GetCan'tAnimDamaged?)
      (if (<= _output_get 0.0)
        (Variables|Default|SetDeath? true :!label _label)
        (Default|DeadPlayer (Variables|Default|GetAs%20AIC%20Boss%20Cursed%20King))
        (Animation|Montage|PlayMontage (Variables|Character|GetMesh) "/Game/ProjectSoul/Animation/Retargeter/AnimRetargeter/AnimPaladinGreatSword_Die_2_Montage.AnimPaladinGreatSword_Die_2_Montage" 0.45
          (:then
            (Collision|SetCollisionEnabled (Variables|Default|GetCapsuleComponent) "NoCollision")
            (Default|EndBarBoss (Variables|Default|GetRefWidgetHp))
            (Audio|PlaySound2D "/Game/ProjectSoul/Sound/CursedTalkDied.CursedTalkDied" 1.0 0.8 0.0 0 0))
          (:OnNotifyEnd
            (Transformation|Teleport "0, 0, 0" "0, 0, 0")
            (Audio|Components|Audio|Stop (Variables|Default|GetRefSound)))))
      (elif (<= _output_get 0.0)
        (goto _label)
        (else
          (Animation|Montage|PlayMontage (Variables|Character|GetMesh) "/Game/ProjectSoul/Animation/Retargeter/AnimRetargeter/AnimPaladinHithit_body_front_Montage.AnimPaladinHithit_body_front_Montage" 0.9))))))

(fn ConstructionScript
  (|CallParentFunction))