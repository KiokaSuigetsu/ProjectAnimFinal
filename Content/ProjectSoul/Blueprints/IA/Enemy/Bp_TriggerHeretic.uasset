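; Trigger volume actor that starts the Heretic boss fight when the player first overlaps its box.
; A DoOnce gate limits it to one firing, after which a valid Heretic reference is set as the player's boss and activated with that player as target.
; It then spawns a 2D sound and a boss health bar widget, stores both on the Heretic, and adds the bar to the viewport.
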(event OnComponentBeginOverlap(Box)
  (params (OverlappedComponent :type Primitive%20Component%20Object%20Reference) (OtherActor :type Actor%20Object%20Reference) (OtherComp :type Primitive%20Component%20Object%20Reference) (OtherBodyIndex :type Integer) (bFromSweep :type Boolean) (SweepResult :type Hit%20Result%20Structure%20%28by%20ref%29))
  (bind _asbp_player (Utilities|Casting|CastToBP_Player OtherActor))
  (Utilities|DoOnce false
    (:Completed
      (bind _heretic (Variables|Default|GetHeretic)
        (:then
          (Variables|/Game/ProjectSoul/Blueprints/Player/BP_Player.BP_Player_C|SetRefBoss _asbp_player _heretic)
          (Default|ActivateBoss _heretic _asbp_player)
          (bind _returnvalue (UserInterface|CreateWidget "/Game/ProjectSoul/Widget/WBP_BossHealthBar.WBP_BossHealthBar_C" 0 _heretic))
          (bind _returnvalue_2 (Audio|SpawnSound2D 0 (Variables|Default|GetVolume%20Multiplier) 1.0 0.0 0))
          (Variables|/Game/ProjectSoul/Blueprints/IA/Enemy/Bp_Heretic.Bp_Heretic_C|SetRefSound _heretic _returnvalue_2)
          (bind _output_get (Variables|/Game/ProjectSoul/Blueprints/IA/Boss/Bp_MainBoss.Bp_MainBoss_C|SetRefWidgetHp _heretic _returnvalue))
          (UserInterface|Viewport|AddtoViewport _output_get 0))
        (:else)))))

(fn ConstructionScript)