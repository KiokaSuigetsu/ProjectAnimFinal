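; Heretic boss enemy that, once activated with a player reference, hands the fight to its AI controller.
; A near-per-frame looping timer keeps it facing the player until stopped.
; Attacks sphere-trace between two scene points, with debug drawing, and damage the hit actor.
; Incoming damage is reduced by defense; hit reactions play only when hittable, and death is just a slowed reaction plus a debug print.
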(event Custom|ActivateBoss
  (params (PlayerRef :type BP%20Player%20Object%20Reference))
  (Variables|Default|SetBossActivate? true)
  (bind _output_get (Variables|Default|SetPlayerRef PlayerRef))
  (bind _output_get_2 (Variables|Default|SetAs%20AIC%20Heretic (.AsAIC%20Heretic (Utilities|Casting|CastToAIC_Heretic (AI|GetAIController self)))))
  (Default|BeginBoss _output_get_2 _output_get)
  (CallFunction|RotatePlayer))

(event Custom|RotatePlayer
  ;[1 1 1] Set/Unset Player to Rotation
  (bind _returnvalue (Utilities|Time|SetTimerbyEvent (delegate Custom|Rotate) 0.001 true))
  (Variables|Default|SetTimerRotate _returnvalue))

(event Custom|Rotate
  ;[1 1 1] Set/Unset Player to Rotation
  (bind _playerref (Variables|Default|GetPlayerRef)
    (:then
      (Transformation|SetActorRotation (Math|Rotator|MakeRotator (.roll (Math|Rotator|FindLookatRotation (Transformation|GetActorLocation) (Transformation|GetActorLocation _playerref))) 0.0 (.yaw (Math|Rotator|FindLookatRotation (Transformation|GetActorLocation) (Transformation|GetActorLocation _playerref))))))
    (:else)))

(event Custom|StopRotatePlayer
  ;[1 1 1] Set/Unset Player to Rotation
  (Utilities|Time|ClearandInvalidateTimerbyHandle (Variables|Default|GetTimerRotate)))

(event Custom|Attack
  (bind (_outhit _returnvalue) (Collision|SphereTraceByChannel (Transformation|GetWorldLocation (Variables|Default|GetScene)) (Transformation|GetWorldLocation (Variables|Default|GetScene1)) 1e+02 "TraceTypeQuery3" false 0 "ForDuration" true "(R=1.000000,G=0.000000,B=0.000000,A=1.000000)" "(R=0.000000,G=1.000000,B=0.000000,A=1.000000)" 3.0))
  (if _returnvalue
    (Game|Damage|ApplyDamage (.HitActor (Collision|BreakHitResult _outhit)) (Variables|Default|GetAtk) 0 0)))

(event Game|Damage|EventAnyDamage
  (params (Damage :type Float%20%28single-precision%29) (DamageType :type Damage%20Type%20Object%20Reference) (InstigatedBy :type Controller%20Object%20Reference) (DamageCauser :type Actor%20Object%20Reference))
  (bind _output_get (Variables|Default|SetHp (.DamageFinalResult (CallFunction|ReductionDamage (Variables|Default|GetHp) Damage (Variables|Default|GetDefense)))))
  (if (Variables|Default|GetHitable?)
    (if (<= _output_get 0.0)
      (Animation|Montage|PlayMontage (Variables|Character|GetMesh) "/Game/Market/AnimationPack/BossyEnemy/Animations/Boss_ReactionHit_F_Montage.Boss_ReactionHit_F_Montage" 0.5
        (:then
          (Development|PrintString "Dead")))
      (else
        (Animation|Montage|PlayMontage (Variables|Character|GetMesh) "/Game/Market/AnimationPack/BossyEnemy/Animations/Boss_ReactionHit_F_Montage.Boss_ReactionHit_F_Montage")))))

(fn ConstructionScript
  (|CallParentFunction))