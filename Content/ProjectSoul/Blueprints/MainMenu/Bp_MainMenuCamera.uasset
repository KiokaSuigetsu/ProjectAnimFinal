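; Main menu camera actor that shows the title/menu widget over a slowly rotating static mesh.
; BeginPlay creates WBP_MainMenu and adds it to the viewport, and Tick steadily yaws the mesh.
; Any key press calls EndTitle on the widget, but only if BeginLoop is already true, and nothing here initially sets it.
; An UpDown timeline for vertical mesh motion exists but never runs.
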(event EventBeginPlay
  (bind _returnvalue (UserInterface|CreateWidget "/Game/ProjectSoul/Widget/WBP_MainMenu.WBP_MainMenu_C"))
  (bind _output_get (Variables|Default|SetRefMainMenuWidget _returnvalue))
  (UserInterface|Viewport|AddtoViewport _output_get 0))

(event EventTick
  (params (DeltaSeconds :type Float%20%28single-precision%29))
  (Transformation|AddRelativeRotation (Variables|Default|GetStaticMesh) (Math|Rotator|MakeRotator 0.0 0.0 (* DeltaSeconds 2e+01)) false false))

(event Input|KeyboardEvents|AnyKey
  (params (Key :type Key%20Structure :default "None"))
  (:Pressed
    (if (Variables|Default|GetBeginLoop?)
      (Variables|Default|SetBeginLoop? true)
      (Default|EndTitle (Variables|Default|GetRefMainMenuWidget)))))

(fn ConstructionScript)