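; Tutorial interactable actor that acts as either an Interact object or a Weapon pickup, chosen by ETypeTuto.
; The construction script shows four skeletal meshes for Interact or one static mesh for Weapon.
; Interaction registers itself on the player, deactivates movement and uses a timeline to turn the player toward it.
; InteractTuto sets the reel mesh or shows the weapon tutorial and equips the weapon, then destroys the actor.
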(event Custom|InteractTuto
  (bind _player_ref (Variables|Default|GetPlayer%20Ref))
  (bind _refwidgetinteface (Variables|/Game/ProjectSoul/Blueprints/Player/BP_Player.BP_Player_C|GetRefWidgetInteface _player_ref))
  (switch Utilities|FlowControl|Switch|SwitchonE_TutoType (Variables|Default|GetE_TypeTuto)
    (:NewEnumerator1
      (Default|SetReelMesh _player_ref))
    (:NewEnumerator4
      (Default|AffTuto _refwidgetinteface (Variables|/Game/ProjectSoul/Widget/WBP_PlayerInterface.WBP_PlayerInterface_C|GetAnimationWeapon _refwidgetinteface))
      (Default|EquipWeapon _player_ref)
      (Variables|/Game/ProjectSoul/Blueprints/Player/BP_Player.BP_Player_C|SetAsWeapon? _player_ref true)))
  (Actor|DestroyActor))

(event EventInteraction
  (params (PlayerRef :type BP%20Player%20Object%20Reference) (ItemRef :type Bp%20Loot%20Object%20Reference) (TutoInteract :type Bp%20Interact%20Tuto%20Object%20Reference))
  (Variables|/Game/ProjectSoul/Blueprints/Player/BP_Player.BP_Player_C|SetInteractTutoRef PlayerRef self)
  (Variables|Default|SetPlayer%20Ref PlayerRef)
  (Components|Activation|Deactivate (Variables|/Script/Engine.Character|GetCharacterMovement PlayerRef))
  (bind _lerpalpha (Timeline|Timeline Play)
    (:Update
      (Default|Rotate PlayerRef PlayerRef self _lerpalpha))))

(fn ConstructionScript
  (bind _staticmesh (Variables|Default|GetStaticMesh))
  (switch Utilities|FlowControl|Switch|SwitchonE_TutoType (Variables|Default|GetE_TypeTuto)
    (:NewEnumerator1
      (Rendering|SetVisibility _staticmesh false false)
      (Rendering|SetVisibility (Variables|Default|GetSkeletalMesh3) true false))
    (:NewEnumerator4
      (Rendering|SetVisibility _staticmesh true false)
      (Rendering|SetVisibility (Variables|Default|GetSkeletalMesh3) false false))))