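; Bp_Tp is a trigger-box actor that starts the player's transition to the Gothic Cathedral level.
; On the player's first overlap with the Box, it shows a loading-screen widget initialized with that level and disables player input.
; It then sets the game instance's current world to the cathedral and copies the cathedral respawn location into the active respawn location.
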(event OnComponentBeginOverlap(Box)
  (params (OverlappedComponent :type Primitive%20Component%20Object%20Reference) (OtherActor :type Actor%20Object%20Reference) (OtherComp :type Primitive%20Component%20Object%20Reference) (OtherBodyIndex :type Integer) (bFromSweep :type Boolean) (SweepResult :type Hit%20Result%20Structure%20%28by%20ref%29))
  (bind _returnvalue (Game|GetGameInstance))
  (bind _asgm_custom_game_instance (Utilities|Casting|CastToGM_CustomGameInstance _returnvalue))
  (Utilities|Casting|CastToBP_Player OtherActor)
  (Development|PrintString "yes")
  (Utilities|FlowControl|DoOnce false
    (:Completed
      (bind _returnvalue_2 (UserInterface|CreateWidget "/Game/ProjectSoul/Widget/WBP_LaodingScreenBegin.WBP_LaodingScreenBegin_C" 0 "Forward" "/Game/Gothic_Cathedral/Maps/Gothic_Cathedral.Gothic_Cathedral"))
      (UserInterface|Viewport|AddtoViewport _returnvalue_2 0)
      (Input|DisableInput (Game|GetPlayerController 0))
      (Variables|/Game/ProjectSoul/Blueprints/GM_CustomGameInstance.GM_CustomGameInstance_C|SetCurrentWorld _asgm_custom_game_instance "/Game/Gothic_Cathedral/Maps/Gothic_Cathedral.Gothic_Cathedral")
      (Variables|/Game/ProjectSoul/Blueprints/GM_CustomGameInstance.GM_CustomGameInstance_C|SetLocationToRespawn _asgm_custom_game_instance (Variables|/Game/ProjectSoul/Blueprints/GM_CustomGameInstance.GM_CustomGameInstance_C|GetLocationToRespawnCathedral _asgm_custom_game_instance)))))

(fn ConstructionScript)