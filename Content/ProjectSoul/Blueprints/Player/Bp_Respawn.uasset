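; Respawn checkpoint Blueprint that sets the player's respawn location when interacted with.
; Interaction deactivates the player's CharacterMovement and runs a Timeline that rotates the player toward the checkpoint.
; In parallel, after a short delay, it stores its Scene component's world location as LocationToRespawn in GM_CustomGameInstance.
; Movement is not reactivated in this graph.
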(event EventInteraction
  (params (PlayerRef :type BP%20Player%20Object%20Reference) (ItemRef :type Bp%20Loot%20Object%20Reference) (TutoInteract :type Bp%20Interact%20Tuto%20Object%20Reference))
  (Utilities|FlowControl|Sequence
    (:then_0
      (Utilities|FlowControl|Delay 0.75)
      (Variables|/Game/ProjectSoul/Blueprints/GM_CustomGameInstance.GM_CustomGameInstance_C|SetLocationToRespawn (.AsGM%20Custom%20Game%20Instance (Utilities|Casting|CastToGM_CustomGameInstance (Game|GetGameInstance))) (Transformation|GetWorldLocation (Variables|Default|GetScene))))
    (:then_1
      (Components|Activation|Deactivate (Variables|/Script/Engine.Character|GetCharacterMovement PlayerRef))
      (bind _lerpalpha (Timeline|Timeline Play)
        (:Update
          (Default|Rotate PlayerRef PlayerRef self _lerpalpha))))))

(fn ConstructionScript)