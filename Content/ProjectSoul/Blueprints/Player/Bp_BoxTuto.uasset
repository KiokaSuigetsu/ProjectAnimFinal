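; Tutorial trigger box that shows a one-time hint when the player overlaps it.
; The ETypeTuto variable picks the widget animation and duration passed to AffTuto on the player's interface widget, with no animation wired for Weapon.
; The box then destroys itself, and the Run and Heal types also set the player's dash and heal flags.
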(event OnComponentBeginOverlap(Box)
  (params (OverlappedComponent :type Primitive%20Component%20Object%20Reference) (OtherActor :type Actor%20Object%20Reference) (OtherComp :type Primitive%20Component%20Object%20Reference) (OtherBodyIndex :type Integer) (bFromSweep :type Boolean) (SweepResult :type Hit%20Result%20Structure%20%28by%20ref%29))
  (bind _e_typetuto (Variables|Default|GetE_TypeTuto))
  (bind _asbp_player (Utilities|Casting|CastToBP_Player OtherActor))
  (Utilities|FlowControl|Sequence
    (:then_0
      (Default|AffTuto (Variables|/Game/ProjectSoul/Blueprints/Player/BP_Player.BP_Player_C|GetRefWidgetInteface _asbp_player) (Utilities|Select :Index _e_typetuto :NewEnumerator0 (Variables|/Game/ProjectSoul/Widget/WBP_PlayerInterface.WBP_PlayerInterface_C|GetAnimationDash (Variables|/Game/ProjectSoul/Blueprints/Player/BP_Player.BP_Player_C|GetRefWidgetInteface _asbp_player)) :NewEnumerator1 (Variables|/Game/ProjectSoul/Widget/WBP_PlayerInterface.WBP_PlayerInterface_C|GetAnimInteract (Variables|/Game/ProjectSoul/Blueprints/Player/BP_Player.BP_Player_C|GetRefWidgetInteface _asbp_player)) :NewEnumerator2 (Variables|/Game/ProjectSoul/Widget/WBP_PlayerInterface.WBP_PlayerInterface_C|GetAnumationAttack (Variables|/Game/ProjectSoul/Blueprints/Player/BP_Player.BP_Player_C|GetRefWidgetInteface _asbp_player)) :NewEnumerator3 (Variables|/Game/ProjectSoul/Widget/WBP_PlayerInterface.WBP_PlayerInterface_C|GetAnimationHeal (Variables|/Game/ProjectSoul/Blueprints/Player/BP_Player.BP_Player_C|GetRefWidgetInteface _asbp_player)) :NewEnumerator4 0) (Utilities|Select :Index _e_typetuto :NewEnumerator0 2.0 :NewEnumerator1 2.0 :NewEnumerator2 5.0 :NewEnumerator3 2.0 :NewEnumerator4 2.0))
      (Actor|DestroyActor))
    (:then_1
      (switch Utilities|FlowControl|Switch|SwitchonE_TutoType (Variables|Default|GetE_TypeTuto)
        (:NewEnumerator0
          (Variables|/Game/ProjectSoul/Blueprints/Player/BP_Player.BP_Player_C|SetAsDash? _asbp_player true))
        (:NewEnumerator3
          (Variables|/Game/ProjectSoul/Blueprints/Player/BP_Player.BP_Player_C|SetAsHeal? _asbp_player true))))))

(fn ConstructionScript)