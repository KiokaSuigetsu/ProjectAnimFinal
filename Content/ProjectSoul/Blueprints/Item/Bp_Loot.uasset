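; Lootable world pickup that the player interacts with; the file handles its feedback and cleanup but grants no item.
; Interaction registers the loot as the player's RefItem, caches the player mesh, deactivates character movement and runs a timeline turning the player toward it.
; LootItem fires once, removing the box, dispersing and deactivating the Niagara effect, attaching NS_OnPlayer to that mesh, clearing RefItem and setting a short lifespan.
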(event Custom|LootItem
  (bind _niagara (Variables|Default|GetNiagara))
  (if (Variables|Default|GetIsLootable?)
    (Variables|Default|SetIsLootable? false)
    (Components|DestroyComponent (Variables|Default|GetBox))
    (Niagara|SetNiagaraVariable(Float) _niagara "ScaleCurve" 1e+03)
    (Niagara|SetNiagaraVariable(Float) _niagara "Noise Strength" 1e+03)
    (Components|Activation|Deactivate _niagara)
    (Actor|SetLifeSpan 5.0)
    (Niagara|SpawnSystemAttached "/Game/ProjectSoul/Particle/OnPlayer/NS_OnPlayer.NS_OnPlayer" (Variables|Default|GetMesh) "None" "0, 0, 0" "0, 0, 0" "KeepRelativeOffset" false)
    (Variables|/Game/ProjectSoul/Blueprints/Player/BP_Player.BP_Player_C|SetRefItem (stale EventInteraction PlayerRef) 0)))

(event EventBeginPlay)

(event Collision|EventActorBeginOverlap
  (params (OtherActor :type Actor%20Object%20Reference)))

(event EventTick
  (params (DeltaSeconds :type Float%20%28single-precision%29)))

(event EventInteraction
  (params (PlayerRef :type BP%20Player%20Object%20Reference) (ItemRef :type Bp%20Loot%20Object%20Reference) (TutoInteract :type Bp%20Interact%20Tuto%20Object%20Reference))
  (Variables|Default|SetMesh (Variables|/Script/Engine.Character|GetMesh PlayerRef))
  (Variables|/Game/ProjectSoul/Blueprints/Player/BP_Player.BP_Player_C|SetRefItem PlayerRef self)
  (Components|Activation|Deactivate (Variables|/Script/Engine.Character|GetCharacterMovement PlayerRef))
  (bind _lerpalpha (Timeline|RotateLerp Play)
    (:Update
      (Default|Rotate PlayerRef PlayerRef self _lerpalpha))))

(fn ConstructionScript)